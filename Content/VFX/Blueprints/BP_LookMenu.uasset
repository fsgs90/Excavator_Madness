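; BP_LookMenu is an actor that shows a preview excavator whose body color can be changed, apparently for a look customization menu.
; On BeginPlay it creates a dynamic material instance on material slot 1 of DisplayExcavator and stores it as BodyMID.
; SetPreviewBodyColor writes the new color to that instance's ColorOverlay parameter, while InitPreviewMaterial duplicates the BeginPlay setup as a callable function.
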(event `self.ReceiveBeginPlay`
  (bind _returnvalue (`PrimitiveComponent.CreateDynamicMaterialInstance` (`self.DisplayExcavator`) 1 null "None"))
  (set `self.BodyMID` _returnvalue))

(fn `InitPreviewMaterial`
  (bind _returnvalue (`PrimitiveComponent.CreateDynamicMaterialInstance` (`self.DisplayExcavator`) 1 null "None"))
  (set `self.BodyMID` _returnvalue))

(fn `SetPreviewBodyColor`
  (params (NewColor :type "LinearColor Structure"))
  (bind _bodymid (`self.BodyMID`))
  (`/Engine/EditorBlueprintResources/StandardMacros.IsValid` _bodymid
    (:`Is Valid`
      (`MaterialInstanceDynamic.SetVectorParameterValue` _bodymid "ColorOverlay" NewColor))))

(fn `UserConstructionScript`)