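; BP_BarrelTowerDestructible is a barrel tower destructible that awards destruction score through the player excavator.
; The player's first overlap with its Box plays a short-lived sound, then resets Score after a delay.
; Each Box end overlap compares the overlapped component, not the other actor, to the player pawn, then adds points and calls CallDestructionTxt on the excavator.
; BeginPlay fills SMArray with placed mesh actors, unused in these graphs.
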(event `self.Box.OnComponentEndOverlap`
  (params (OverlappedComponent :type "PrimitiveComponent Object Reference") (OtherActor :type "Actor Object Reference") (OtherComp :type "PrimitiveComponent Object Reference") (OtherBodyIndex :type Integer))
  (if (!= OverlappedComponent (`GameplayStatics.GetPlayerPawn` 0))
    (`KismetSystemLibrary.PrintString` "Add Destruction Score!")
    (set `self.Score` (+ (`self.Score`) 100.0))
    (bind _asbp_player_excavator (cast `/Game/Player/BP_Player_Excavator` (`GameplayStatics.GetPlayerPawn` 0)))
    (`/Game/Player/BP_Player_Excavator.CallDestructionTxt` _asbp_player_excavator (`self.Score`))))

(event `self.ReceiveBeginPlay`
  (set `self.SMArray` (`|MakeArray` (`self.StaticMeshActor_UAID_200B740F32BD6CBD02_1271895151`) (`self.StaticMeshActor_UAID_200B740F32BD6CBD02_1271902154`) (`self.StaticMeshActor_UAID_200B740F32BD6CBD02_1271906156`) (`self.StaticMeshActor_UAID_200B740F32BD6CBD02_1271908157`) (`self.StaticMeshActor_UAID_200B740F32BD6CBD02_1271905155`) (`self.StaticMeshActor_UAID_200B740F32BD6CBD02_1271900153`))))

(event `self.Box.OnComponentBeginOverlap`
  (params (OverlappedComponent :type "PrimitiveComponent Object Reference") (OtherActor :type "Actor Object Reference") (OtherComp :type "PrimitiveComponent Object Reference") (OtherBodyIndex :type Integer) (bFromSweep :type Boolean) (SweepResult :type "HitResult Structure (by ref)"))
  (if (== OtherActor (`GameplayStatics.GetPlayerPawn` 0))
    (`/Engine/EditorBlueprintResources/StandardMacros.DoOnce` false
      (:`Completed`
        (bind _returnvalue (`AddComponent|NODE_AddAudioComponent-1`))
        (`AudioComponent.Play` _returnvalue 0.4)
        (`KismetSystemLibrary.Delay` 1.2)
        (`ActorComponent.K2_DestroyComponent` _returnvalue)
        (set `self.Score` 0.0)))))

(fn `UserConstructionScript`)