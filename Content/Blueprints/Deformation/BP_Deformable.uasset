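; Deformable car actor that dents and flattens at runtime, using Geometry Script on a dynamic mesh copied from a static mesh.
; Debounced player hits add capped damage, applying Perlin noise and limited sine warps.
; Player roof overlaps flatten the mesh by clamped scaling, deform it, and trigger sound and camera shake.
; Debug keys drive damage, flattening and off-origin crushing; front, back and side trigger logic is disconnected.
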(event `self.DeformableMesh.OnComponentHit`
  (params (HitComponent :type "PrimitiveComponent Object Reference") (OtherActor :type "Actor Object Reference") (OtherComp :type "PrimitiveComponent Object Reference") (NormalImpulse :type "Vector Structure") (Hit :type "HitResult Structure (by ref)"))
  ; Detect Collision And Select Geo
  (`|ExecutionSequence`
    (:`then_0`
      (`/Engine/EditorBlueprintResources/StandardMacros.DoOnce` false :!label _label
        (:`Completed`
          (if (== OtherActor (`GameplayStatics.GetPlayerPawn` 0))
            (`|ExecutionSequence`
              (:`then_1`
                (`KismetSystemLibrary.PrintString` "PlayerCollision"))
              (:`then_2`
                (`self.Take Damage` 0.1)))))))
    (:`then_1`
      (`KismetSystemLibrary.Delay` 0.5)
      (goto _label :!via `Reset`))))

(event `self.ReceiveBeginPlay`
  ; Set Variables On Begin Play
  (bind _returnvalue (`BaseDynamicMeshComponent.GetDynamicMesh` (`self.DeformableMesh`)))
  (set `self.Target Mesh` _returnvalue))

(event `Take Damage`
  (params (DamageToTake :type "Float (double-precision)"))
  (bind _damage (`self.Damage`))
  ; Take Damage
  (if (< _damage 1.0)
    (bind _output_get (set `self.Damage` (+ _damage DamageToTake)))
    (`KismetSystemLibrary.PrintString` (`KismetStringLibrary.Conv_DoubleToString` _output_get))
    (`self.Deform`)))

(event `Deform`
  (bind _target_mesh (`self.Target Mesh`))
  ; Deformation Logic
  (`GeometryScriptLibrary_MeshDeformFunctions.ApplyPerlinNoiseToMesh2` _target_mesh (struct) (make `GeometryScriptPerlinNoiseOptions` (make `GeometryScriptPerlinNoiseLayerOptions` 5.0 0.1)))
  (if (< (`self.CurrentCrunch`) (`self.CrunchLimit`))
    (`GeometryScriptLibrary_MeshDeformFunctions.ApplyMathWarpToMesh` _target_mesh (struct) "SinWave1D" (make `GeometryScriptMathWarpOptions` 5.0))
    (set `self.CurrentCrunch` (+ (`self.CurrentCrunch`) 0.1))
    (`KismetSystemLibrary.PrintString` "MeshDeformed")))

(event `Key|NumPadNine`
  (params (Key :type "Key Structure"))
  ;[0.002398 0.4487 1 0.5] Manually Increase Deformation
  (:`Pressed`
    (`self.CrushCar` (-100.0 -40.0 40.0) (0.0 0.01 0.0))))

(event `Key|Add`
  (params (Key :type "Key Structure"))
  ;[0.002398 0.4487 1 0.5] Manually Increase Deformation
  (:`Pressed`
    (`self.Take Damage` 0.1)))

(event `FlattenCar`
  (bind _scale (`self.Scale`))
  (bind (_scale_x _scale_y _scale_z) (`KismetMathLibrary.BreakVector` (`self.Scale`)))
  ;[0 0.7345 1 0.5] Flatten Car Logic
  (if (> _scale_z 0.7)
    (`GeometryScriptLibrary_MeshTransformFunctions.ScaleMesh` (`self.Target Mesh`) _scale)
    (set `self.Scale` (- _scale (`self.FlattenScale`)))
    (`KismetSystemLibrary.PrintString` "Flattening Car")))

(event `Key|Subtract`
  (params (Key :type "Key Structure"))
  ;[0.002398 0.4487 1 0.5] Manually Increase Deformation
  (:`Pressed`
    (`self.FlattenCar`)))

(event `Key|NumPadEight`
  (params (Key :type "Key Structure"))
  ;[0.002398 0.4487 1 0.5] Manually Increase Deformation
  (:`Pressed`
    (`self.CrushCar` (-100.0 40.0 40.0) (0.0 0.01 0.0))))

(event `Key|Multiply`
  (params (Key :type "Key Structure"))
  ;[0.002398 0.4487 1 0.5] Manually Increase Deformation
  (:`Pressed`
    (`self.CrushCar` (-200.0 0.0 40.0) (`self.CrushScale`))))

(event `CrushCar`
  (params (CompressionOrigin :type "Vector Structure") (CompressionScale :type "Vector Structure"))
  (bind (_scale_x _scale_y) (`KismetMathLibrary.BreakVector` (`self.Scale`)))
  ;[0 0.4858 0.9583 0.5] Crush Car Logic
  (if (and (> _scale_x 0.9) (> _scale_y 0.9))
    (bind _output_get (set `self.Scale` (- (`self.Scale`) CompressionScale)))
    (`GeometryScriptLibrary_MeshTransformFunctions.ScaleMesh` (`self.Target Mesh`) _output_get CompressionOrigin)
    (`KismetSystemLibrary.PrintString` "Crushing Car")))

(event `Key|Divide`
  (params (Key :type "Key Structure"))
  ;[0.002398 0.4487 1 0.5] Manually Increase Deformation
  (:`Pressed`
    (`self.CrushCar` (0.0 0.0 40.0) (`self.CrushScale`))))

(event `self.COL_Roof.OnComponentBeginOverlap`
  (params (OverlappedComponent :type "PrimitiveComponent Object Reference") (OtherActor :type "Actor Object Reference") (OtherComp :type "PrimitiveComponent Object Reference") (OtherBodyIndex :type Integer) (bFromSweep :type Boolean) (SweepResult :type "HitResult Structure (by ref)"))
  ;[0.15 0.1462 0 0.5] Only Active Deformation For Now
  (if (== OtherActor (`GameplayStatics.GetPlayerPawn` 0))
    (`|ExecutionSequence`
      (:`then_0`
        (`/Engine/EditorBlueprintResources/StandardMacros.DoOnce` false :!label _label_2
          (:`Completed`
            (`self.FlattenCar`)
            (`self.Deform`)
            (bind _returnvalue (`GameplayStatics.SpawnSound2D` "/Game/Blueprints/Deformation/CrushSFX.CrushSFX" 1.0 1.0 0.0 null))
            (`AudioComponent.Play` _returnvalue 0.0)
            ;[0.1248 0.02739 0.15 0.5] Camera Shake
            (bind _asbp_vehicle_adv_player_controller (cast `/Game/VehicleTemplate/Blueprints/BP_VehicleAdvPlayerController` (`GameplayStatics.GetPlayerController` 0)))
            (`PlayerController.ClientStartCameraShake` :`self` _asbp_vehicle_adv_player_controller :`Shake` "/Game/Blueprints/BP_CameraShaker.BP_CameraShaker_C")
            (`KismetSystemLibrary.Delay` 5.0))))
      (:`then_1`
        (`KismetSystemLibrary.Delay` 5.0)
        (goto _label_2 :!via `Reset`)))))

(event `self.COL_Front.OnComponentBeginOverlap`
  (params (OverlappedComponent :type "PrimitiveComponent Object Reference") (OtherActor :type "Actor Object Reference") (OtherComp :type "PrimitiveComponent Object Reference") (OtherBodyIndex :type Integer) (bFromSweep :type Boolean) (SweepResult :type "HitResult Structure (by ref)"))
  ;[0.00849 0.309 1 0.5] CarSquash
)

(event `self.COL_Back.OnComponentBeginOverlap`
  (params (OverlappedComponent :type "PrimitiveComponent Object Reference") (OtherActor :type "Actor Object Reference") (OtherComp :type "PrimitiveComponent Object Reference") (OtherBodyIndex :type Integer) (bFromSweep :type Boolean) (SweepResult :type "HitResult Structure (by ref)"))
  ;[0.00849 0.309 1 0.5] CarSquash
)

(event `self.COL_Right.OnComponentBeginOverlap`
  (params (OverlappedComponent :type "PrimitiveComponent Object Reference") (OtherActor :type "Actor Object Reference") (OtherComp :type "PrimitiveComponent Object Reference") (OtherBodyIndex :type Integer) (bFromSweep :type Boolean) (SweepResult :type "HitResult Structure (by ref)"))
  ;[0.00849 0.309 1 0.5] CarSquash
)

(event `self.COL_Left.OnComponentBeginOverlap`
  (params (OverlappedComponent :type "PrimitiveComponent Object Reference") (OtherActor :type "Actor Object Reference") (OtherComp :type "PrimitiveComponent Object Reference") (OtherBodyIndex :type Integer) (bFromSweep :type Boolean) (SweepResult :type "HitResult Structure (by ref)"))
  ;[0.00849 0.309 1 0.5] CarSquash
)

(fn `UserConstructionScript`
  (bind _deformablemesh (`self.DeformableMesh`))
  ; Initialize Mesh
  (bind _returnvalue (`BaseDynamicMeshComponent.GetDynamicMesh` (`self.DeformableMesh`)))
  (`GeometryScriptLibrary_StaticMeshFunctions.CopyMeshFromStaticMeshV2` (`self.From Static Mesh Asset`) _returnvalue
    (:`Success`
      (`PrimitiveComponent.SetMaterial` _deformablemesh 0 "/Game/Materials/MaterialsOLD/Mat_3_Inst.Mat_3_Inst")
      (`PrimitiveComponent.SetMaterial` _deformablemesh 1 "/Game/Materials/MaterialsOLD/window_cracked.window_cracked"))))