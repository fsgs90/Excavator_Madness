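; Thrown steel barrel bomb actor that explodes when its collision sphere overlaps any actor other than the player pawn.
; A DoOnce-guarded overlap prints the other actor's name, hides the barrel and fire meshes or effects, and plays explosion sound.
; It then fires the bomb Niagara effect, shakes the player's camera, calls destruction text on the excavator pawn, and destroys itself after a short delay.
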(event `self.COL_Sphere.OnComponentBeginOverlap`
  (params (OverlappedComponent :type "PrimitiveComponent Object Reference") (OtherActor :type "Actor Object Reference") (OtherComp :type "PrimitiveComponent Object Reference") (OtherBodyIndex :type Integer) (bFromSweep :type Boolean) (SweepResult :type "HitResult Structure (by ref)"))
  ; Barrel Explosion - Modifies particles, plays sound and destroys actor
  (if (not (== OtherActor (`GameplayStatics.GetPlayerPawn` 0)))
    (`KismetSystemLibrary.PrintString` (`KismetSystemLibrary.GetDisplayName` OtherActor))
    (`/Engine/EditorBlueprintResources/StandardMacros.DoOnce` false
      (:`Completed`
        (`SceneComponent.SetHiddenInGame` (`self.SM_Barrel`) true false)
        (`SceneComponent.SetHiddenInGame` (`self.NS_FireBarrel`) true false)
        (`AudioComponent.Play` (`self.SFX_Explosion`) 0.0)
        (`|ExecutionSequence`
          (:`then_0`
            (`ActorComponent.Activate` (`self.NS_Bomb`) false)
            (`KismetSystemLibrary.Delay` 1.0)
            (`self.K2_DestroyActor`))
          (:`then_1`
            (bind _asbp_vehicle_adv_player_controller (cast `/Game/VehicleTemplate/Blueprints/BP_VehicleAdvPlayerController` (`GameplayStatics.GetPlayerController` 0)))
            (`PlayerController.ClientStartCameraShake` :`self` _asbp_vehicle_adv_player_controller :`Shake` "/Game/Blueprints/Camera/BP_CamShake_Landing.BP_CamShake_Landing_C" :`PlaySpace` "World"))
          (:`then_2`
            (bind _asbp_player_excavator (cast `/Game/Player/BP_Player_Excavator` (`GameplayStatics.GetPlayerPawn` 0)))
            (`/Game/Player/BP_Player_Excavator.CallDestructionTxt` _asbp_player_excavator 250.0)))))))

(fn `UserConstructionScript`)