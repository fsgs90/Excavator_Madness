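; BP_BarrelPlayerSocket is a barrel actor with fire effects and an overlap sphere, named for a socket on the player.
; Its sphere overlap event is empty, so the explosion logic is disconnected and never runs.
; That unused chain would hide the barrel on non-player contact, play bomb effects and sound, shake the camera, call the excavator's destruction text and destroy the actor after a delay.
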(event `self.COL_Sphere.OnComponentBeginOverlap`
  (params (OverlappedComponent :type "PrimitiveComponent Object Reference") (OtherActor :type "Actor Object Reference") (OtherComp :type "PrimitiveComponent Object Reference") (OtherBodyIndex :type Integer) (bFromSweep :type Boolean) (SweepResult :type "HitResult Structure (by ref)"))
  ; Barrel Explosion - Modifies particles, plays sound and destroys actor
)

(fn `UserConstructionScript`)