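; Deformable car prop that dents, flattens and crushes at runtime using Geometry Script on a dynamic mesh copied from a static mesh.
; Player hits, throttled by DoOnce and a delay, add capped damage that triggers Perlin noise and a limited sine-wave warp.
; Debug keys add damage or step-scale the mesh to flatten or crush it.
; The roof hit only cycles its DoOnce, and vertex selection and twist/bend experiments are unconnected.
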(event `self.ReceiveBeginPlay`
  (bind _returnvalue (`BaseDynamicMeshComponent.GetDynamicMesh` (`self.DeformableMesh`)))
  (set `self.Target Mesh` _returnvalue))

(event `self.DeformableMesh.OnComponentHit`
  (params (HitComponent :type "PrimitiveComponent Object Reference") (OtherActor :type "Actor Object Reference") (OtherComp :type "PrimitiveComponent Object Reference") (NormalImpulse :type "Vector Structure") (Hit :type "HitResult Structure (by ref)"))
  ; Detect Collision And Select Geo
  (`|ExecutionSequence`
    (:`then_0`
      (`/Engine/EditorBlueprintResources/StandardMacros.DoOnce` false :!label _label
        (:`Completed`
          (if (== OtherActor (`GameplayStatics.GetPlayerPawn` 0))
            (`|ExecutionSequence`
              (:`then_1`
                (`KismetSystemLibrary.PrintString` "PlayerCollision"))
              (:`then_2`
                (`self.Take Damage` 0.1)))))))
    (:`then_1`
      (`KismetSystemLibrary.Delay` 0.5)
      (goto _label :!via `Reset`))))

(event `self.COL_Roof.OnComponentHit`
  (params (HitComponent :type "PrimitiveComponent Object Reference") (OtherActor :type "Actor Object Reference") (OtherComp :type "PrimitiveComponent Object Reference") (NormalImpulse :type "Vector Structure") (Hit :type "HitResult Structure (by ref)"))
  ; CarSquash
  (`|ExecutionSequence`
    (:`then_0`
      (`/Engine/EditorBlueprintResources/StandardMacros.DoOnce` false :!label _label_2))
    (:`then_1`
      (`KismetSystemLibrary.Delay` 5.0)
      (goto _label_2 :!via `Reset`))))

(event `Take Damage`
  (params (DamageToTake :type "Float (double-precision)"))
  (bind _damage (`self.Damage`))
  ; Take Damage
  (if (< _damage 1.0)
    (bind _output_get (set `self.Damage` (+ _damage DamageToTake)))
    (`KismetSystemLibrary.PrintString` (`KismetStringLibrary.Conv_DoubleToString` _output_get))
    (`self.Deform`)))

(event `Deform`
  (bind _target_mesh (`self.Target Mesh`))
  ; Deformation Logic
  (`GeometryScriptLibrary_MeshDeformFunctions.ApplyPerlinNoiseToMesh2` _target_mesh (struct) (make `GeometryScriptPerlinNoiseOptions` (make `GeometryScriptPerlinNoiseLayerOptions` 1.0 0.1)))
  (if (< (`self.CurrentCrunch`) (`self.CrunchLimit`))
    (`GeometryScriptLibrary_MeshDeformFunctions.ApplyMathWarpToMesh` _target_mesh (struct) "SinWave1D" (make `GeometryScriptMathWarpOptions` 5.0))
    (set `self.CurrentCrunch` (+ (`self.CurrentCrunch`) 0.1))
    (`KismetSystemLibrary.PrintString` "MeshDeformed")))

(event `FlattenCar`
  (bind _scale (`self.Scale`))
  (bind (_scale_x _scale_y _scale_z) (`KismetMathLibrary.BreakVector` (`self.Scale`)))
  ; Flatten Car Logic
  (if (> _scale_z 0.7)
    (`GeometryScriptLibrary_MeshTransformFunctions.ScaleMesh` (`self.Target Mesh`) _scale)
    (set `self.Scale` (- _scale (`self.FlattenScale`)))
    (`KismetSystemLibrary.PrintString` "Flattening Car")))

(event `Key|Add`
  (params (Key :type "Key Structure"))
  ; Manually Increase Deformation
  (:`Pressed`
    (`self.Take Damage` 0.1)))

(event `Key|Subtract`
  (params (Key :type "Key Structure"))
  ; Manually Increase Deformation
  (:`Pressed`
    (`self.FlattenCar`)))

(event `Key|Multiply`
  (params (Key :type "Key Structure"))
  ; Manually Increase Deformation
  (:`Pressed`
    (`self.CrushCar`)))

(event `CrushCar`
  (bind _scale_x (`KismetMathLibrary.BreakVector` (`self.Scale`)))
  (bind _scale (`self.Scale`))
  ; Flatten Car Logic
  (if (> _scale_x 0.7)
    (set `self.Scale` (- _scale (`self.CrushScale`)))
    (`GeometryScriptLibrary_MeshTransformFunctions.ScaleMesh` (`self.Target Mesh`) _scale)
    (`KismetSystemLibrary.PrintString` "Crushing Car")))

(fn `UserConstructionScript`
  ; Initialize Mesh
  (bind _returnvalue (`BaseDynamicMeshComponent.GetDynamicMesh` (`self.DeformableMesh`)))
  (`GeometryScriptLibrary_StaticMeshFunctions.CopyMeshFromStaticMeshV2` (`self.From Static Mesh Asset`) _returnvalue))