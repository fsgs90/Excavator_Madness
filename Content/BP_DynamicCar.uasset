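; BP_DynamicCar is a Geometry Script actor that procedurally deforms a mesh, presumably a car given its name.
; Its construction script copies InputMesh into the DynamicMeshComponent, then chains a twist warp, two Perlin noise passes and a bend warp.
; Variables drive the twist, the first noise pass and the bend, while the second noise pass uses default options.
; The event graph holds no active logic.
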(fn `UserConstructionScript`
  (bind _returnvalue (`BaseDynamicMeshComponent.GetDynamicMesh` (`self.DynamicMeshComponent`)))
  (bind _returnvalue_2 (`GeometryScriptLibrary_StaticMeshFunctions.CopyMeshFromStaticMeshV2` (`self.Input Mesh`) _returnvalue)
    (:`Success`
      (bind _returnvalue_3 (`GeometryScriptLibrary_MeshDeformFunctions.ApplyTwistWarpToMesh` _returnvalue_2 (make `GeometryScriptTwistWarpOptions` true) (struct) (`self.Twist Angle`) (`self.Twist Extent`)))
      (bind _returnvalue_4 (`GeometryScriptLibrary_MeshDeformFunctions.ApplyPerlinNoiseToMesh2` _returnvalue_3 (struct) (make `GeometryScriptPerlinNoiseOptions` (make `GeometryScriptPerlinNoiseLayerOptions` (`self.Magnitude`) (`self.Frequency`)) false)))
      (bind _returnvalue_5 (`GeometryScriptLibrary_MeshDeformFunctions.ApplyPerlinNoiseToMesh2` _returnvalue_4))
      (`GeometryScriptLibrary_MeshDeformFunctions.ApplyBendWarpToMesh` _returnvalue_5 (struct) (struct) (`self.Bend Angle`) (`self.Bend Extent`)))))